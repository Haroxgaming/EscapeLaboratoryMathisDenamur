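; Interactable sliding double door in the Science Lab that toggles open and closed while CanOpen is set.
; Interact alternates through a FlipFlop, playing or reversing a Timeline that slides the two door meshes apart on local Y.
; Closing also calls CheckWorldGravity on every RailingPlatform132_Blueprint, provided the player character is a BP_Body.
; The construction script destroys the Collision component on doors that cannot open.
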(event EventInteract
  ;[0 0.3281 0] SecurityBreach0X00CF52
  (if (Variables|Default|GetCanOpen)
    (Utilities|FlowControl|FlipFlop
      (:A
        (bind _open (Timeline|Timeline Play)
          (:Update
            (Transformation|SetRelativeLocation (Variables|Default|GetLabDoor03B) (Math|Vector|MakeVector 0.0 (* _open 1e+02) 0.0) false false)
            (Transformation|SetRelativeLocation (Variables|Default|GetLabDoor03A) (Math|Vector|MakeVector 0.0 (* (* _open 1e+02) -1.0) 0.0) false false))))
      (:B
        ;[1 0 0] SecurityBreachFixed
        (Utilities|FlowControl|Sequence
          (:then_0
            (Timeline|Timeline Reverse))
          (:then_1
            (Utilities|Casting|CastToBP_Body (Game|GetPlayerCharacter 0))
            (bind _outactors (Actor|GetAllActorsOfClass "/Game/ScienceLab/Blueprints/RailingPlatform132_Blueprint.RailingPlatform132_Blueprint_C"))
            (for _array_element _outactors
              (Default|CheckWorldGravity _array_element))))))))

(fn ConstructionScript
  (if (not (Variables|Default|GetCanOpen))
    (Components|DestroyComponent (Variables|Default|GetCollision))))