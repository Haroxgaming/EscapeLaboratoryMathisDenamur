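; Two-panel sliding lab door that toggles open and closed when interacted with, if CanOpen is set.
; A FlipFlop alternates playing and reversing a timeline that slides the panels in opposite directions along local Y.
; The construction script offsets the panels by DoorPosition, assigns three configurable materials to panels and jamb, and destroys the Collision component on doors that cannot open.
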(event EventInteract
  ;[0 0.3281 0] SecurityBreach0X00CF52
  (if (Variables|Default|GetCanOpen)
    (Utilities|FlowControl|FlipFlop
      (:A
        (bind _open (Timeline|Timeline Play)
          (:Update
            (Transformation|SetRelativeLocation (Variables|Default|GetLabDoor03B) (Math|Vector|MakeVector 0.0 (* _open 1e+02) 0.0) false false)
            (Transformation|SetRelativeLocation (Variables|Default|GetLabDoor03A) (Math|Vector|MakeVector 0.0 (* (* _open 1e+02) -1.0) 0.0) false false))))
      (:B
        (Timeline|Timeline Reverse)))))

(fn ConstructionScript
  (bind _materail2 (Variables|Default|GetMaterail2))
  (bind _doorposition (Variables|Default|GetDoorPosition))
  (bind _materail1 (Variables|Default|GetMaterail1))
  (bind _labdoor03a (Variables|Default|GetLabDoor03A))
  (bind _labdoor03b (Variables|Default|GetLabDoor03B))
  ;[1 1 1] Movement
  (Transformation|AddRelativeLocation _labdoor03b (Math|Vector|MakeVector 0.0 _doorposition 0.0) false false)
  (Transformation|AddRelativeLocation _labdoor03a (Math|Vector|MakeVector 0.0 (* _doorposition -1.0) 0.0) false false)
  ;[1 1 1] Materail
  (Rendering|Material|SetMaterial _labdoor03b 0 _materail1)
  (Rendering|Material|SetMaterial (Variables|Default|GetLabDoorjamb03) 1 _materail2)
  (Rendering|Material|SetMaterial _labdoor03a 0 _materail2)
  (Rendering|Material|SetMaterial _labdoor03a 1 _materail1)
  (Rendering|Material|SetMaterial _labdoor03b 2 (Variables|Default|GetMaterail3))
  (if (not (Variables|Default|GetCanOpen))
    (Components|DestroyComponent (Variables|Default|GetCollision))))