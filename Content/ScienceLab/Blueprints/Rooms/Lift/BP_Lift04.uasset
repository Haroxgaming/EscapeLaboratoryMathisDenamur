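; BP_Lift04 is a lift door with two hinged panels that swing open automatically for a BP_Body.
; On overlap, if the referenced lift's Top state differs from the door's, it calls JoinPlayer on the lift and waits before opening.
; A timeline rotates the panels in mirrored yaw and reverses on end overlap.
; The construction script sets initial angle and material, and destroys the trigger when CanOpen is false.
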(event OnComponentBeginOverlap(Collision)
  (params (OverlappedComponent :type Primitive%20Component%20Object%20Reference) (OtherActor :type Actor%20Object%20Reference) (OtherComp :type Primitive%20Component%20Object%20Reference) (OtherBodyIndex :type Integer) (bFromSweep :type Boolean) (SweepResult :type Hit%20Result%20Structure%20%28by%20ref%29))
  ;[0 0.3281 0] AutoOpenAndColseDoor
  (Utilities|Casting|CastToBP_Body OtherActor)
  (if (!= (Variables|/Game/ScienceLab/Blueprints/Rooms/Lift/BP_Lift03.BP_Lift03_C|GetTop (Variables|Default|GetLift%20Ref)) (Variables|Default|GetTop?))
    (Default|JoinPlayer (Variables|Default|GetLift%20Ref))
    (Utilities|FlowControl|Delay 5.0)
    (bind _open (Timeline|Timeline Play)
      (:Update
        (Transformation|SetRelativeRotation (Variables|Default|GetLift02Door02) (Math|Rotator|MakeRotator 0.0 0.0 (* _open 45.0)) false false)
        (Transformation|SetRelativeRotation (Variables|Default|GetLift02Door01) (Math|Rotator|MakeRotator 0.0 0.0 (* (* _open 45.0) -1.0)) false false)))
    (else
      (Timeline|Timeline Play))))

(event OnComponentEndOverlap(Collision)
  (params (OverlappedComponent :type Primitive%20Component%20Object%20Reference) (OtherActor :type Actor%20Object%20Reference) (OtherComp :type Primitive%20Component%20Object%20Reference) (OtherBodyIndex :type Integer))
  ;[0 0.3281 0] AutoOpenAndColseDoor
  (Utilities|Casting|CastToBP_Body OtherActor)
  (bind _open (Timeline|Timeline Reverse)
    (:Update
      (Transformation|SetRelativeRotation (Variables|Default|GetLift02Door02) (Math|Rotator|MakeRotator 0.0 0.0 (* _open 45.0)) false false)
      (Transformation|SetRelativeRotation (Variables|Default|GetLift02Door01) (Math|Rotator|MakeRotator 0.0 0.0 (* (* _open 45.0) -1.0)) false false))))

(fn ConstructionScript
  (bind _doorposition (Variables|Default|GetDoorPosition))
  (bind _lift02door01 (Variables|Default|GetLift02Door01))
  ;[1 1 1] Movement
  (Transformation|SetRelativeRotation (Variables|Default|GetLift02Door02) (Math|Rotator|MakeRotator 0.0 0.0 _doorposition) false false)
  (Transformation|SetRelativeRotation _lift02door01 (Math|Rotator|MakeRotator 0.0 0.0 (* _doorposition -1.0)) false false)
  ;[1 1 1] Material
  (Rendering|Material|SetMaterial _lift02door01 0 (Variables|Default|GetMaterial))
  (if (not (Variables|Default|GetCanOpen))
    (Components|DestroyComponent (Variables|Default|GetCollision))))